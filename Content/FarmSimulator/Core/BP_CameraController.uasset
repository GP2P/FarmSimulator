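; Player camera controller for the farm simulator, a character-based rig with a spring arm that supports moving, strafing, orbiting, tilting and zooming.
; Movement input follows control-yaw only, orbit adds controller yaw, and pitch rotates the spring arm within tilt limits.
; Zoom changes the clamped arm length, then rescales max walk speed relative to minimum zoom so the camera travels faster when zoomed out.
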(event Custom|CameraOrbit
  (params (Magnitude :type Float%20%28double-precision%29))
  (Pawn|Input|AddControllerYawInput (* (Variables|Default|GetOrbitSpeed) Magnitude)))

(event Custom|CameraMove
  (params (Magnitude :type Float%20%28double-precision%29))
  (Pawn|Input|AddMovementInput (Math|Vector|GetForwardVector (Math|Rotator|MakeRotator 0.0 0.0 (.Yaw (Math|Rotator|BreakRotator (Pawn|GetControlRotation :!class /Script/Engine.Pawn))))) Magnitude false))

(event Custom|CameraStrafe
  (params (Magnitude :type Float%20%28double-precision%29))
  (Pawn|Input|AddMovementInput (Math|Vector|GetRightVector (Math|Rotator|MakeRotator 0.0 0.0 (.Yaw (Math|Rotator|BreakRotator (Pawn|GetControlRotation :!class /Script/Engine.Pawn))))) Magnitude false))

(event Custom|CameraZoom
  (params (Magnitude :type Float%20%28double-precision%29))
  (Variables|/Script/Engine.SpringArmComponent|SetTargetArmLength (Variables|Default|GetSpringArm) (Math|Float|Clamp(Float) (+ (Variables|/Script/Engine.SpringArmComponent|GetTargetArmLength (Variables|Default|GetSpringArm)) (* Magnitude (Variables|Default|GetZoomSpeed))) (Variables|Default|GetZoomMin) (Variables|Default|GetZoomMax)))
  (CallFunction|UpdateMoveSpeed))

(event Custom|CameraPitch
  (params (Magnitude :type Float%20%28double-precision%29))
  (bind _springarm (Variables|Default|GetSpringArm))
  (bind _returnvalue (Transformation|GetWorldRotation _springarm))
  (bind (_roll _pitch _yaw) (Math|Rotator|BreakRotator _returnvalue))
  (Transformation|SetWorldRotation (Variables|Default|GetSpringArm) (Math|Rotator|MakeRotator _roll (Math|Float|ClampAngle (+ (* Magnitude (Variables|Default|GetOrbitSpeed)) (.Pitch (Math|Rotator|BreakRotator (Transformation|GetWorldRotation (Variables|Default|GetSpringArm))))) (Variables|Default|GetCameraTiltMin) (Variables|Default|GetCameraTiltMax)) _yaw) false false))

(event EventBeginPlay
  (Variables|Default|SetMoveSpeedDefault (Variables|/Script/Engine.CharacterMovementComponent|GetMaxWalkSpeed (Variables|Character|GetCharacterMovement)))
  (CallFunction|UpdateMoveSpeed))

(fn ConstructionScript)

(fn UpdateMoveSpeed
  (Variables|/Script/Engine.CharacterMovementComponent|SetMaxWalkSpeed (Variables|Character|GetCharacterMovement) (* (/ (Variables|/Script/Engine.SpringArmComponent|GetTargetArmLength (Variables|Default|GetSpringArm)) (Variables|Default|GetZoomMin)) (Variables|Default|GetMoveSpeedDefault))))