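; Worker manager for the farm simulator that tracks registered houses, their active workers, and current versus maximum population.
; Registering a house adds its capacity and workers to the totals; removing one tries to rehouse its workers and destroys those it cannot place.
; Workers join a house by grid coordinates, falling back to the first house that accepts them.
; RemoveWorker is empty, and RegisterNewWorker seeks housing only when population is at or above maximum, otherwise destroying the worker.
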(event EventBeginPlay)

(event Collision|EventActorBeginOverlap
  (params (OtherActor :type Actor%20Object%20Reference)))

(event EventTick
  (params (DeltaSeconds :type Float%20%28single-precision%29)))

(fn ConstructionScript)

(fn RegisterHouse
  (params (House :type GO%20House%20Base%20Object%20Reference))
  (Utilities|Array|Add (Variables|Default|GetRegisteredHouses) House)
  (Variables|Default|SetMaxPopulation (+ (Variables|Default|GetMaxPopulation) (Variables|/Game/FarmSimulator/GameObjects/Houses/Core/GO_House_Base.GO_House_Base_C|GetMaxPopulation House)))
  (Variables|Default|SetCurrentPopulation (+ (Variables|Default|GetCurrentPopulation) (Variables|/Game/FarmSimulator/GameObjects/Houses/Core/GO_House_Base.GO_House_Base_C|GetCurrentPopulation House)))
  (for _array_element (Variables|/Game/FarmSimulator/GameObjects/Houses/Core/GO_House_Base.GO_House_Base_C|GetActiveWorkers House)
    (Utilities|Array|Add (Variables|Default|GetActiveWorkers) _array_element)))

(fn RemoveHouse
  (params (House :type GO%20House%20Base%20Object%20Reference))
  (bind _returnvalue (Utilities|Array|RemoveItem (Variables|Default|GetRegisteredHouses) House))
  (if _returnvalue
    (Variables|Default|SetMaxPopulation (- (Variables|Default|GetMaxPopulation) (Variables|/Game/FarmSimulator/GameObjects/Houses/Core/GO_House_Base.GO_House_Base_C|GetMaxPopulation House)))
    (for _array_element (Variables|/Game/FarmSimulator/GameObjects/Houses/Core/GO_House_Base.GO_House_Base_C|GetActiveWorkers House) ; Reassign workers if possible, destroy on capacity full
      (bind _assignsuccess (CallFunction|ReassignExistingWorker _array_element))
      (if (not _assignsuccess)
        (if (>= (Variables|Default|GetCurrentPopulation) (Variables|Default|GetMaxPopulation))
          (bind _returnvalue_2 (Utilities|Array|RemoveItem (Variables|Default|GetActiveWorkers) _array_element))
          (if _returnvalue_2
            _
            (else
              (Development|PrintString "Error: couldn't remove worker")))
          (else
            (Development|PrintString "Error: have capacity but can't reassign")))
        (Math|Integer|DecrementInt (Variables|Default|GetCurrentPopulation)
          (:%20%20
            (Actor|DestroyActor _array_element)))))
    (else
      (Development|PrintString "Removed house not registered"))))

(fn RegisterNewWorker
  (params (Worker :type BP%20Worker%20Base%20Object%20Reference))
  (if (>= (Variables|Default|GetCurrentPopulation) (Variables|Default|GetMaxPopulation))
    (for _array_element (Variables|Default|GetRegisteredHouses)
      (bind _assignsuccess (Default|AssignWorker _array_element Worker))
      (if _assignsuccess
        (Utilities|Array|Add (Variables|Default|GetActiveWorkers) Worker)
        (Math|Integer|IncrementInt (Variables|Default|GetCurrentPopulation)
          (:%20%20
            (return true)))))
    (Development|PrintString "Error: can't add to any house")
    (return false)
    (else
      (Actor|DestroyActor Worker)
      (Development|PrintString "Capacity Full")
      (return false))))

(fn ReassignExistingWorker
  (params (Worker :type BP%20Worker%20Base%20Object%20Reference))
  (for _array_element (Variables|Default|GetRegisteredHouses)
    (bind _assignsuccess (Default|AssignWorker _array_element Worker))
    (if _assignsuccess
      (return true)))
  (Development|PrintString "Can't add to any house")
  (return false))

(fn RemoveWorker)

(fn AssignWorkertoHouse
  (params (Worker :type BP%20Worker%20Base%20Object%20Reference) (House%20Coord%20X :type Integer) (House%20Coord%20Y :type Integer))
  ;[1 1 1] Find House with the Coords
  (for _array_element (Variables|Default|GetRegisteredHouses)
    (if (and (== (Variables|/Game/FarmSimulator/GameObjects/Core/BP_GameObject_Base.BP_GameObject_Base_C|GetGrid%20Coord%20X _array_element) House%20Coord%20X) (== (Variables|/Game/FarmSimulator/GameObjects/Core/BP_GameObject_Base.BP_GameObject_Base_C|GetGrid%20Coord%20Y _array_element) House%20Coord%20Y))
      (bind _assignsuccess (Default|AssignWorker _array_element Worker))
      (if _assignsuccess
        (Utilities|Array|Add (Variables|Default|GetActiveWorkers) Worker)
        (Math|Integer|IncrementInt (Variables|Default|GetCurrentPopulation))
        (else
          (CallFunction|RegisterNewWorker Worker) ; Assign to other houses if failed
        )))))