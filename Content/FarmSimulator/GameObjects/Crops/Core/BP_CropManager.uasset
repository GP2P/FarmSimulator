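; BP_CropManager is the central manager that drives crop growth for registered farm tiles in the farm simulator.
; Farm tiles are added to and removed from the RegisteredCrops array through register and remove functions, with registration returning the array index.
; Once StartGrowing fires, a one-second Delay loop calls CropGrowth with a random increment on every valid entry.
; Each pass runs all at once so crop indices stay stable.
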(event Custom|StartGrowing
  ;[1 1 1] Increment matureness every second
  (Utilities|FlowControl|Delay 1.0 :!label _label)
  (CallFunction|IncrementMatureness)
  (goto _label))

(fn ConstructionScript)

(fn IncrementMatureness
  (for _array_element (Variables|Default|GetRegistered%20Crops) ; Execute all at once, else crops index will change
    (Utilities|IsValid _array_element
      (:Is%20Valid
        (Default|CropGrowth _array_element (Math|Random|RandomFloatinRange 0.0 1.0))))))

(fn RegisterFarmTile
  (params (FarmTile :type GO%20Farm%20Tile%20Object%20Reference))
  (bind _returnvalue (Utilities|Array|Add (Variables|Default|GetRegistered%20Crops) FarmTile))
  (return _returnvalue))

(fn RemoveFarmTile
  (params (Farm%20Tile :type GO%20Farm%20Tile%20Object%20Reference))
  (Utilities|Array|RemoveItem (Variables|Default|GetRegistered%20Crops) Farm%20Tile))