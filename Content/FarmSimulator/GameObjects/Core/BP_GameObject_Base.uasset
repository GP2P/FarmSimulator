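; Base actor for farm simulator game objects, providing optional hover and click selection plus registration with BP_GridManager.
; BeginPlay binds cursor events based on the clickable and hoverable flags; clicks toggle selection outside placement mode and update BP_PlayerController's ClickedActors list.
; Hover and selection share a custom-depth highlight on all static meshes, which stays on while either is active.
; GO_OnSpawn and GO_OnDestroy register and remove the object from the grid manager.
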(event Custom|OnMouseClick
  (params (TouchedActor :type Actor%20Object%20Reference) (ButtonPressed :type Key%20Structure :default "None"))
  ;[1 1 1] Only work if not in placement mode
  (bind _returnvalue (Actor|GetActorOfClass "/Game/FarmSimulator/Core/BP_PlayerController.BP_PlayerController_C"))
  (if (not (Variables|/Game/FarmSimulator/Core/BP_PlayerController.BP_PlayerController_C|GetInPlacementMode _returnvalue))
    (Variables|HoverandClick|SetIs%20Clicked (not (Variables|HoverandClick|GetIs%20Clicked)))
    (if (Variables|HoverandClick|GetIs%20Clicked)
      (bind _returnvalue_2 (Actor|GetActorOfClass "/Game/FarmSimulator/Core/BP_PlayerController.BP_PlayerController_C"))
      (Utilities|Array|Add (Variables|/Game/FarmSimulator/Core/BP_PlayerController.BP_PlayerController_C|GetClickedActors _returnvalue_2) self)
      (if (not (Variables|HoverandClick|GetIs%20Hovered))
        (for _array_element (Actor|GetComponentsByClass "/Script/Engine.StaticMeshComponent")
          (Rendering|SetRenderCustomDepth _array_element true)))
      (else
        (bind _returnvalue_3 (Actor|GetActorOfClass "/Game/FarmSimulator/Core/BP_PlayerController.BP_PlayerController_C"))
        (Utilities|Array|RemoveItem (Variables|/Game/FarmSimulator/Core/BP_PlayerController.BP_PlayerController_C|GetClickedActors _returnvalue_3) self)
        (if (not (Variables|HoverandClick|GetIs%20Hovered))
          (for _array_element_2 (Actor|GetComponentsByClass "/Script/Engine.StaticMeshComponent")
            (Rendering|SetRenderCustomDepth _array_element_2 false)))))))

(event Custom|OnMouseHoverStart
  (params (TouchedActor :type Actor%20Object%20Reference))
  (Variables|HoverandClick|SetIs%20Hovered true)
  (if (not (Variables|HoverandClick|GetIs%20Clicked))
    (for _array_element (Actor|GetComponentsByClass "/Script/Engine.StaticMeshComponent")
      (Rendering|SetRenderCustomDepth _array_element true))))

(event Custom|OnMouseHoverEnd
  (params (TouchedActor :type Actor%20Object%20Reference))
  (Variables|HoverandClick|SetIs%20Hovered false)
  (if (not (Variables|HoverandClick|GetIs%20Clicked))
    (for _array_element (Actor|GetComponentsByClass "/Script/Engine.StaticMeshComponent")
      (Rendering|SetRenderCustomDepth _array_element false))))

(event EventBeginPlay
  (if (Variables|GameObjectInfo|GetIs%20Clickable)
    (EventDispatchers|BindEventtoOnClicked (delegate Custom|OnMouseClick)))
  (if (Variables|GameObjectInfo|GetIs%20Hoverable)
    (EventDispatchers|BindEventtoOnBeginCursorOver (delegate Custom|OnMouseHoverStart))
    (EventDispatchers|BindEventtoOnEndCursorOver (delegate Custom|OnMouseHoverEnd))))

(fn ConstructionScript)

(fn GOonSpawn
  (bind _returnvalue (Actor|GetActorOfClass "/Game/FarmSimulator/GameObjects/Core/BP_GridManager.BP_GridManager_C"))
  (Default|RegisterGameObject _returnvalue self))

(fn GOonDestroy
  (bind _returnvalue (Actor|GetActorOfClass "/Game/FarmSimulator/GameObjects/Core/BP_GridManager.BP_GridManager_C"))
  (Default|RemoveGameObject _returnvalue self))