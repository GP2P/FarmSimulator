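; BP_GridManager builds and queries the farm game's square grid of BP_GridCell actors, centered on the world origin.
; PopulateGrid spawns cells into a row-major GridCells array, and PopulateCellNeighbors links each to its north, south, east and west neighbors by index arithmetic.
; Lookups map grid coordinates or world positions to cells or snapped centers, using MyTruncate to handle negatives.
; UpdateGridCount changes the width, then saves and reloads "GameMap" through BP_SaveGameManager.
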(fn ConstructionScript)

(fn PopulateGrid
  (Utilities|Array|Clear (Variables|Default|GetGrid%20Cells))
  (bind _grid_start_offset (|CalculateOffset))
  (bind _y_coord (|YLoop)
    (:LoopBody
      (bind _x_coord (|XLoop)
        (:LoopBody
          (|SpawnActor (|CalculatePosition _x_coord _y_coord _grid_start_offset) _x_coord _y_coord))))))

(fn GetClosestGridPos
  (params (Input :type Vector))
  (bind (_x _y) (Math|Vector|BreakVector Input))
  (bind _cell_width (Variables|Default|GetCell%20Width))
  (bind _cell_width_2 (Variables|Default|GetCell%20Width))
  (bind _output (CallFunction|MyTruncate (/ _x (Variables|Default|GetCell%20Width))))
  (bind _output_2 (CallFunction|MyTruncate (/ _y (Variables|Default|GetCell%20Width))))
  (return (Math|Vector|MakeVector (Math|Conversions|ToFloat(Integer) (+ (* _output _cell_width_2) (/ _cell_width_2 2))) (Math|Conversions|ToFloat(Integer) (+ (* _output_2 _cell_width) (/ _cell_width 2))) 0.0)))

(fn MyTruncate
  (params (Input :type Float%20%28double-precision%29))
  (bind _returnvalue (Math|Float|Truncate Input))
  (if (< Input 0.0)
    (return (+ _returnvalue -1))
    (else
      (return _returnvalue))))

(fn PopulateCellNeighbors
  (for (_array_element _array_index) (Variables|Default|GetGrid%20Cells)
    (|SetSouthNeighbors _array_element _array_index)
    (|SetNorthNeighbors _array_index _array_element)
    (|SetEastNeighbors _array_index _array_element)
    (|SetWestNeighbors _array_index _array_element)))

(fn GetClosestGridCell
  (params (Input :type Vector))
  (bind (_x _y) (Math|Vector|BreakVector Input))
  (bind _output (CallFunction|MyTruncate (/ _x (Variables|Default|GetCell%20Width))))
  (bind _output_2 (CallFunction|MyTruncate (/ _y (Variables|Default|GetCell%20Width))))
  (return (Utilities|Array|Get(acopy) (Variables|Default|GetGrid%20Cells) (+ (* (Math|Integer|Clamp(Integer) (+ _output_2 (/ (Variables|Default|GetGrid%20Width) 2)) 0 (Variables|Default|GetGrid%20Width)) (Variables|Default|GetGrid%20Width)) (Math|Integer|Clamp(Integer) (+ (/ (Variables|Default|GetGrid%20Width) 2) _output) 0 (Variables|Default|GetGrid%20Width))))))

(fn GetGridCellfromGridCoord
  (params (GridCoordX :type Integer) (GridCoordY :type Integer))
  (return (Utilities|Array|Get(acopy) (Variables|Default|GetGrid%20Cells) (+ GridCoordX (* GridCoordY (Variables|Default|GetGrid%20Width))))))

(fn UpdateGridCount
  (params (GridCount :type Integer))
  (Variables|Default|SetGrid%20Width GridCount)
  (bind _returnvalue (Actor|GetActorOfClass "/Game/FarmSimulator/Core/BP_SaveGameManager.BP_SaveGameManager_C"))
  (Default|SaveGame _returnvalue "GameMap")
  (Default|LoadSaveGame _returnvalue "GameMap"))