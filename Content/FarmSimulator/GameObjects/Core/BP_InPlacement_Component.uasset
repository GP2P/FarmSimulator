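; Placement component for farm simulator preview objects that decides whether the owner can be built at its location and shows the result.
; UpdatePlaceableState, run on BeginPlay, checks origin-centered grid bounds, using width for both axes, then queries BP_GridManager's closest cell.
; Crop previews require an empty farm tile, while other objects require an unoccupied cell.
; It swaps all static mesh materials to placeable, invalid or the crop preview's own material.
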(event EventBeginPlay
  (CallFunction|UpdatePlaceableState))

(fn UpdatePlaceableState
  (bind _returnvalue (Components|GetOwner))
  (bind _returnvalue_2 (Components|GetOwner))
  (bind _returnvalue_3 (Actor|GetComponentsByClass _returnvalue_2 "/Script/Engine.StaticMeshComponent"))
  (bind _returnvalue_4 (Transformation|GetActorLocation _returnvalue))
  (bind (_x _y) (Math|Vector|BreakVector _returnvalue_4))
  (bind _returnvalue_5 (Actor|GetActorOfClass "/Game/FarmSimulator/GameObjects/Core/BP_GridManager.BP_GridManager_C"))
  (LocalVariables|SetGridManager _returnvalue_5)
  ;[1 1 1] Check if build inside scope
  (if (and (<= (Math|Float|Absolute(Float) _x) (/ (* (Variables|/Game/FarmSimulator/GameObjects/Core/BP_GridManager.BP_GridManager_C|GetGrid%20Width (LocalVariables|GetGridManager)) (Variables|/Game/FarmSimulator/GameObjects/Core/BP_GridManager.BP_GridManager_C|GetCell%20Width (LocalVariables|GetGridManager))) 2.0)) (<= (Math|Float|Absolute(Float) _y) (/ (* (Variables|/Game/FarmSimulator/GameObjects/Core/BP_GridManager.BP_GridManager_C|GetGrid%20Width (LocalVariables|GetGridManager)) (Variables|/Game/FarmSimulator/GameObjects/Core/BP_GridManager.BP_GridManager_C|GetCell%20Width (LocalVariables|GetGridManager))) 2.0)))
    (bind _output (Default|GetClosestGridCell (LocalVariables|GetGridManager) _returnvalue_4))
    (LocalVariables|SetClosestGridCell _output)
    ;[1 1 1] Check if is Crop Preview
    (bind _asbp_game_object_base (Utilities|Casting|CastToBP_GameObject_Base (Components|GetOwner)))
    (if (Utilities|Enum|Equal(Enum) (Variables|/Game/FarmSimulator/GameObjects/Core/BP_GameObject_Base.BP_GameObject_Base_C|GetObject%20Type _asbp_game_object_base) "NewEnumerator4")
      (if (and (Utilities|Enum|Equal(Enum) (Variables|/Game/FarmSimulator/GameObjects/Core/BP_GridCell.BP_GridCell_C|GetObject%20Type (LocalVariables|GetClosestGridCell)) "NewEnumerator3") (Variables|/Game/FarmSimulator/GameObjects/Core/BP_GridCell.BP_GridCell_C|GetIs%20Occupied (LocalVariables|GetClosestGridCell)))
        ;[1 1 1] Check if Farm Tile Empty
        (bind _asgo_farm_tile (Utilities|Casting|CastToGO_FarmTile (Variables|/Game/FarmSimulator/GameObjects/Core/BP_GridCell.BP_GridCell_C|GetGame%20Object (LocalVariables|GetClosestGridCell)))
          (:then
            (if (Utilities|Enum|Equal(Enum) (Variables|/Game/FarmSimulator/GameObjects/GO_FarmTile.GO_FarmTile_C|GetCrop%20Type _asgo_farm_tile) "NewEnumerator0")
              (Variables|Default|SetIs%20Placement%20Valid true)
              ;[1 1 1] Set Crop Preview Material
              (bind _asgo_crop_preview (Utilities|Casting|CastToGO_CropPreview_Base (Components|GetOwner))
                (:then
                  (for _array_element (Actor|GetComponentsByClass (Components|GetOwner) "/Script/Engine.StaticMeshComponent")
                    (for _index (range 0 (- (Utilities|Array|Length (Rendering|Material|GetMaterials _array_element)) 1))
                      (Rendering|Material|SetMaterial _array_element _index (Utilities|Array|Get(acopy) (Variables|/Game/FarmSimulator/GameObjects/GO_CropPreview_Base.GO_CropPreview_Base_C|GetCropPreviewMaterials _asgo_crop_preview)))
                      (Rendering|SetVisibility _array_element true false)))
                  (return))
                (:CastFailed
                  _))
              (else
                (Variables|Default|SetIs%20Placement%20Valid false) ; Farm Tile Occupied
              )))
          (:CastFailed
            _))
        (else
          (Variables|Default|SetIs%20Placement%20Valid false) ; Is Crop Preview but not on Farm Tile
        ))
      (else
        ;[1 1 1] Check if Grid is occupied
        (Variables|Default|SetIs%20Placement%20Valid (not (Variables|/Game/FarmSimulator/GameObjects/Core/BP_GridCell.BP_GridCell_C|GetIs%20Occupied (LocalVariables|GetClosestGridCell))))))
    (else
      (Variables|Default|SetIs%20Placement%20Valid false)))
  ;[1 1 1] Change Material
  (if (Variables|Default|GetIs%20Placement%20Valid)
    (for _array_element_2 _returnvalue_3
      (for _index_2 (range 0 (- (Utilities|Array|Length (Rendering|Material|GetMaterials _array_element_2)) 1))
        (Rendering|Material|SetMaterial _array_element_2 _index_2 "/Game/FarmSimulator/MaterialLibrary/PlaceableMaterial.PlaceableMaterial")
        (Rendering|SetVisibility _array_element_2 true false)))
    (return)
    (else
      (for _array_element_3 _returnvalue_3
        (for _index_3 (range 0 (- (Utilities|Array|Length (Rendering|Material|GetMaterials _array_element_3)) 1))
          (Rendering|Material|SetMaterial _array_element_3 _index_3 "/Game/FarmSimulator/MaterialLibrary/InvalidMaterial.InvalidMaterial")
          (Rendering|SetVisibility _array_element_3 true false)))
      (return))))