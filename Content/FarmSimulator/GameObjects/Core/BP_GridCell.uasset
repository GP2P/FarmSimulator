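; BP_GridCell is one cell of the farm simulator's grid, tracking whether it is occupied and by which game object.
; Binding stores the object and its type, treating the default type as empty.
; Deleting resets the cell and destroys the object, first removing farm tiles from BP_CropManager's registered crops for one object type.
; An unused debug helper tints the four neighbor cells' planes by direction when the cell is occupied.
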(event Custom|ChangePlaneMaterial
  (params (Material :type Material%20Object%20Reference))
  (Rendering|Material|SetMaterial (Variables|Default|GetPlane) 0 Material))

(fn ConstructionScript)

(fn BindGameObject
  (params (GameObject :type BP%20Game%20Object%20Base%20Object%20Reference))
  (if (Utilities|Enum|Equal(Enum) (Variables|/Game/FarmSimulator/GameObjects/Core/BP_GameObject_Base.BP_GameObject_Base_C|GetObject%20Type GameObject) "NewEnumerator0")
    (Variables|Default|SetIs%20Occupied false)
    (else
      (Variables|Default|SetIs%20Occupied true)
      (Variables|Default|SetObject%20Type (Variables|/Game/FarmSimulator/GameObjects/Core/BP_GameObject_Base.BP_GameObject_Base_C|GetObject%20Type GameObject))
      (Variables|Default|SetGame%20Object GameObject))))

(fn DeleteGameObject
  (if (Utilities|Enum|Equal(Enum) (Variables|Default|GetObject%20Type) "NewEnumerator3")
    (bind _returnvalue (Actor|GetActorOfClass "/Game/FarmSimulator/GameObjects/Crops/Core/BP_CropManager.BP_CropManager_C"))
    (bind _asgo_farm_tile (Utilities|Casting|CastToGO_FarmTile (Variables|Default|GetGame%20Object))
      (:then
        (Utilities|Array|RemoveItem (Variables|/Game/FarmSimulator/GameObjects/Crops/Core/BP_CropManager.BP_CropManager_C|GetRegistered%20Crops _returnvalue) _asgo_farm_tile))
      (:CastFailed
        _)))
  (LocalVariables|SetOriginal%20Game%20Object (Variables|Default|GetGame%20Object))
  (Variables|Default|SetIs%20Occupied false)
  (Variables|Default|SetObject%20Type "NewEnumerator0")
  (Variables|Default|SetGame%20Object 0)
  (Actor|DestroyActor (LocalVariables|GetOriginal%20Game%20Object))
  (return))

(fn ShowNeighbors
  (bind _neighbor_north (Variables|Default|GetNeighbor%20North))
  (bind _neighbor_south (Variables|Default|GetNeighbor%20South))
  (bind _neighbor_west (Variables|Default|GetNeighbor%20West))
  (bind _neighbor_east (Variables|Default|GetNeighbor%20East))
  (if (Variables|Default|GetIs%20Occupied)
    (Utilities|IsValid _neighbor_north
      (:Is%20Valid
        (CallFunction|ChangePlaneMaterial _neighbor_north "/Game/FarmSimulator/MaterialLibrary/Debug/M_Red.M_Red"))
      (:Is%20Not%20Valid
        _))
    (Utilities|IsValid _neighbor_west
      (:Is%20Valid
        (CallFunction|ChangePlaneMaterial _neighbor_west "/Game/FarmSimulator/MaterialLibrary/Debug/M_Yellow.M_Yellow"))
      (:Is%20Not%20Valid
        _))
    (Utilities|IsValid _neighbor_east
      (:Is%20Valid
        (CallFunction|ChangePlaneMaterial _neighbor_east "/Game/FarmSimulator/MaterialLibrary/Debug/M_Green.M_Green"))
      (:Is%20Not%20Valid
        _))
    (Utilities|IsValid _neighbor_south
      (:Is%20Valid
        (CallFunction|ChangePlaneMaterial _neighbor_south "/Game/FarmSimulator/MaterialLibrary/Debug/M_Blue.M_Blue")))))