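; BP_Clickable_Component is an actor component in the farm simulator that makes its owning actor respond to mouse clicks and hovering.
; On BeginPlay it binds to the owner's click event, then caches its static mesh and binds cursor-over events if one exists.
; Each click toggles IsClicked and swaps the mesh's first material between placeable and invalid.
; Hovering toggles the mesh's Render Custom Depth flag.
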(event Custom|OnMouseClick
  (params (TouchedActor :type Actor%20Object%20Reference) (ButtonPressed :type Key%20Structure :default "None"))
  (Variables|Default|SetIs%20Clicked (not (Variables|Default|GetIs%20Clicked)))
  (Variables|Default|GetStaticMeshRef
    (:then
      (if (Variables|Default|GetIs%20Clicked)
        (Rendering|Material|SetMaterial (Variables|Default|GetStaticMeshRef) 0 "/Game/FarmSimulator/MaterialLibrary/PlaceableMaterial.PlaceableMaterial")
        (else
          (Rendering|Material|SetMaterial (Variables|Default|GetStaticMeshRef) 0 "/Game/FarmSimulator/MaterialLibrary/InvalidMaterial.InvalidMaterial"))))
    (:else)))

(event Custom|OnMouseHoverStart
  (params (TouchedActor :type Actor%20Object%20Reference))
  (Rendering|SetRenderCustomDepth (Variables|Default|GetStaticMeshRef) true))

(event Custom|OnMouseHoverEnd
  (params (TouchedActor :type Actor%20Object%20Reference))
  (Rendering|SetRenderCustomDepth (Variables|Default|GetStaticMeshRef) false))

(event EventBeginPlay
  (bind _returnvalue (Components|GetOwner))
  (bind _returnvalue_2 (Actor|GetComponentbyClass _returnvalue "/Script/Engine.StaticMeshComponent"))
  (EventDispatchers|BindEventtoOnClicked (Components|GetOwner) (delegate Custom|OnMouseClick))
  (Utilities|IsValid _returnvalue_2
    (:Is%20Valid
      (Variables|Default|SetStaticMeshRef _returnvalue_2)
      (EventDispatchers|BindEventtoOnBeginCursorOver (Components|GetOwner) (delegate Custom|OnMouseHoverStart))
      (EventDispatchers|BindEventtoOnEndCursorOver (Components|GetOwner) (delegate Custom|OnMouseHoverEnd)))))